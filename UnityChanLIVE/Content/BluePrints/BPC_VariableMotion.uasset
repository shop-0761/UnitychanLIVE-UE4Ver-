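; Actor component that makes its owning StaticMeshActor swing back and forth with a variable, sine-driven rotation.
; On BeginPlay it casts and caches the owner, then each Tick adds a world rotation around that actor's right vector.
; The step combines Amplitude, Speed and a game-time sine, randomly reduced per frame by Randomness, and is not scaled by delta time.
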(event EventBeginPlay
  (bind _asstatic_mesh_actor (Utilities|Casting|CastToStaticMeshActor (Components|GetOwner self)))
  (Variables|Default|SetStaticMeshActor _asstatic_mesh_actor))

(event EventTick
  (params (DeltaSeconds :type Float%20%28single-precision%29))
  (bind _staticmeshactor (Variables|Default|GetStaticMeshActor)
    (:then
      (Class|Actor|AddActorWorldRotation (Variables|Default|GetStaticMeshActor) (Math|Vector|RotatorfromAxisandAngle (Transformation|GetActorRightVector _staticmeshactor) (* (Variables|Default|GetAmplitude) (- 1.0 (* (Variables|Default|Getrandomness) (Math|Random|RandomFloat))) (* (Variables|Default|GetSpeed) (* (Math|Trig|Sin(Radians) (* (Utilities|Time|GetGameTimeinSeconds) 0.5)) 1.2))))))
    (:else)))