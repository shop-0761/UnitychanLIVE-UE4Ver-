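; BP_Laser is a reusable laser effect actor with an animated skeletal mesh that stays hidden until activated.
; Activate, skipped when the actor sits at the world origin, shows the mesh, starts its jitter motion component and plays the laser montage.
; A LifeTime timer then calls Reset, which hides and deactivates both components and detaches the actor instead of destroying it.
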(event Custom|Reset
  (Rendering|SetVisibility (Variables|Default|GetLaser) false false)
  (Components|Activation|SetActive (Variables|Default|GetLaser) false false)
  (Transformation|DetachFromActor "KeepRelative" "KeepRelative" "KeepRelative"))

(event EventBeginPlay
  (bind _aslaser_anim_bp (Utilities|Casting|CastToLaserAnimBP (Components|SkeletalMesh|GetAnimInstance (Variables|Default|GetLaser))))
  (Variables|Default|SetAnimBP _aslaser_anim_bp)
  (Rendering|SetVisibility (Variables|Default|GetLaser) false false))

(event EventActivate
  (if (Math|Vector|NotEqual(Vector) (Transformation|GetActorLocation) "0, 0, 0" 1.0)
    (Rendering|SetVisibility (Variables|Default|GetLaser) true false)
    (Components|Activation|SetActive (Variables|Default|GetLaser) true true)
    (Animation|Montage|MontagePlay (Variables|Default|GetAnimBP) "/Game/Meshes/SkeletalMesh/LaserMontage.LaserMontage" 1.0 "Duration" 0.0)
    (Utilities|Time|SetTimerbyEvent (delegate Custom|Reset) (Variables|Default|GetLifeTime))))

(fn ConstructionScript
  (Rendering|SetVisibility (Variables|Default|GetLaser) false false))