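; BPC_Spray is a component that turns a spray particle effect on and off according to how fast a bone on its owner moves.
; On BeginPlay it attaches the emitter to the target bone of the owner's first skeletal mesh.
; Each tick it compares the bone's displacement since the last tick against SprayThreshold.
; Two cross-resetting DoOnce gates make activation and deactivation fire only on threshold crossings, without resetting the particles.
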(event EventBeginPlay
  (bind _self self)
  (bind _returnvalue (Components|GetOwner _self))
  (bind _returnvalue_2 (Actor|GetComponentsByClass _returnvalue "/Script/Engine.SkeletalMeshComponent"))
  (if (> (Utilities|Array|Length _returnvalue_2) 0)
    (Variables|Default|SetSkeletalMesh (Utilities|Array|Get(acopy) _returnvalue_2))
    (Variables|Default|SetPreLocation (Transformation|GetSocketLocation (Variables|Default|GetSkeletalMesh) (Variables|Default|GetTargetBone)))
    (bind _returnvalue_3 (Effects|SpawnEmitterAttached (Variables|Default|GetParticleEmitter) (Variables|Default|GetSkeletalMesh) (Variables|Default|GetTargetBone) "0, 0, 0" "0, 0, 0" "KeepRelativeOffset" false))
    (Variables|Default|SetSprayParticle _returnvalue_3)))

(event EventTick
  (params (DeltaSeconds :type Float%20%28single-precision%29))
  (bind _sprayparticle (Variables|Default|GetSprayParticle))
  (Utilities|FlowControl|Sequence
    (:then_0
      (if (>= (Math|Vector|VectorLength (- (Transformation|GetSocketLocation (Variables|Default|GetSkeletalMesh) (Variables|Default|GetTargetBone)) (Variables|Default|GetPreLocation))) (Variables|Default|GetSprayThreshold))
        (Utilities|FlowControl|DoOnce false :!label _label
          (:Completed
            (Components|Activation|SetActive _sprayparticle true false)
            (goto _label_2 Reset)))
        (else
          (Utilities|FlowControl|DoOnce false :!label _label_2
            (:Completed
              (Components|Activation|SetActive _sprayparticle false false)
              (goto _label Reset))))))
    (:then_1
      (Variables|Default|SetPreLocation (Transformation|GetSocketLocation (Variables|Default|GetSkeletalMesh) (Variables|Default|GetTargetBone))))))