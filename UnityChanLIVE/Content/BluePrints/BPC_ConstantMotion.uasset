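; BPC_ConstantMotion is a component that keeps its owning StaticMeshActor continuously spinning.
; BeginPlay casts and caches the owner, so other actor types get no motion.
; Each Tick adds a relative rotation to the mesh component about the actor's up vector, scaled by Velocity and delta time.
; Randomness scales a per-frame random reduction of that speed.
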(event EventBeginPlay
  (bind _asstatic_mesh_actor (Utilities|Casting|CastToStaticMeshActor (Components|GetOwner self)))
  (Variables|Default|SetStaticMeshActor _asstatic_mesh_actor))

(event EventTick
  (params (DeltaSeconds :type Float%20%28single-precision%29))
  (bind _staticmeshactor (Variables|Default|GetStaticMeshActor)
    (:then
      (Transformation|AddRelativeRotation (Variables|/Script/Engine.StaticMeshActor|GetStaticMeshComponent (Variables|Default|GetStaticMeshActor)) (Math|Vector|RotatorfromAxisandAngle (Transformation|GetActorUpVector _staticmeshactor) (* (Variables|Default|GetVelocity) (- 1.0 (* (Variables|Default|GetRandomness) (Math|Random|RandomFloat))) DeltaSeconds)) false false))
    (:else)))