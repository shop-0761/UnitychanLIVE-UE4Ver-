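; Actor component that prototypes spring-bone secondary motion for the UnityChan character's hair tail.
; MakeSpringBones builds a spring chain from the J_B_HairTail bones, with per-bone sphere colliders on spine and arms.
; UpdateSpring moves each tip by Verlet integration at fixed length, then writes blended look-at rotations into the AnimBP.
; Unfinished: Tick is empty, calls to both routines are disconnected, and collision push-out is unwired.
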(event Custom|MakeSpringBones
  (bind _returnvalue (Utilities|String|MakeLiteralString "J_B_HairTail_00 
J_B_HairTail_01 
J_B_HairTail_02 
J_B_HairTail_03 
J_B_HairTail_04 
J_B_HairTail_04_end"))
  (bind _str_springcollider (Utilities|Struct|MakeSTR_SpringCollider "Character1_LeftArm" 12.0))
  (bind _str_springcollider_2 (Utilities|Struct|MakeSTR_SpringCollider "Character1_Spine2" 15.0))
  (bind _str_springcollider_3 (Utilities|Struct|MakeSTR_SpringCollider "Character1_Spine1" 15.0))
  (bind _str_springcollider_4 (Utilities|Struct|MakeSTR_SpringCollider "Character1_RightArm" 12.0))
  (bind _skeletalmesh (Variables|Default|GetSkeletalMesh))
  (bind _returnvalue_2 (Utilities|String|ParseIntoArray _returnvalue " 
"))
  (bind _array (Utilities|Array|MakeArray _str_springcollider_2))
  (bind _array_2 (Utilities|Array|MakeArray _str_springcollider_2 _str_springcollider _str_springcollider_4 _str_springcollider_3))
  (bind _str_springcolliders (Utilities|Struct|MakeSTR_SpringColliders _array))
  (bind _str_springcolliders_2 (Utilities|Struct|MakeSTR_SpringColliders _array_2))
  (for _index (range 0 (- (Utilities|Array|Length _returnvalue_2) 2))
    (Utilities|Array|Add (Variables|Default|GetSpringBone_J_B_HairTail) (Utilities|Struct|MakeSTR_SpringBone (Utilities|String|StringToName (Utilities|Array|Get(acopy) _returnvalue_2 _index)) (Transformation|GetSocketLocation _skeletalmesh (Utilities|String|StringToName (Utilities|Array|Get(acopy) _returnvalue_2 (+ _index 1)))) (Transformation|GetSocketLocation _skeletalmesh (Utilities|String|StringToName (Utilities|Array|Get(acopy) _returnvalue_2 (+ _index 1)))) 0.01 0.4 "0.001000,0.000000,-0.001000" (Math|Vector|VectorLength (- (Transformation|GetSocketLocation _skeletalmesh (Utilities|String|StringToName (Utilities|Array|Get(acopy) _returnvalue_2 (+ _index 1)))) (Transformation|GetSocketLocation _skeletalmesh (Utilities|String|StringToName (Utilities|Array|Get(acopy) _returnvalue_2 _index))))) (Utilities|Array|Get(acopy) (Variables|/Game/UnityChan/Animations/UnityChanAnimBP.UnityChanAnimBP_C|GetB_HairTailRotations (Variables|Default|GetAnimBP)) _index) (Utilities|Struct|BreakSTR_SpringColliders (Utilities|Array|Get(acopy) (Utilities|Array|MakeArray _str_springcolliders _str_springcolliders _str_springcolliders _str_springcolliders_2 _str_springcolliders_2) _index))))))

(event EventBeginPlay
  (bind _self self)
  (bind _returnvalue (Components|GetOwner _self))
  (bind _returnvalue_2 (Actor|GetComponentsByClass _returnvalue "/Script/Engine.SkeletalMeshComponent"))
  (if (> (Utilities|Array|Length _returnvalue_2) 0)
    (bind _output_get (Variables|Default|SetSkeletalMesh (Utilities|Array|Get(acopy) _returnvalue_2)))
    (bind _asunity_chan_anim_bp (Utilities|Casting|CastToUnityChanAnimBP (Components|SkeletalMesh|GetAnimInstance _output_get)))
    (Variables|Default|SetAnimBP _asunity_chan_anim_bp)))

(event EventTick
  (params (DeltaSeconds :type Float%20%28single-precision%29)))

(fn UpdateSpring
  (bind _returnvalue (Utilities|Time|GetWorldDeltaSeconds))
  (bind _animbp (Variables|Default|GetAnimBP))
  (bind _skeletalmesh (Variables|Default|GetSkeletalMesh))
  (bind _returnvalue_2 (Math|Float|Square _returnvalue))
  (bind _b_hairtailrotations (Variables|/Game/UnityChan/Animations/UnityChanAnimBP.UnityChanAnimBP_C|GetB_HairTailRotations _animbp))
  (for (_array_element _array_index) (Variables|Default|GetSpringBone_J_B_HairTail)
    (Utilities|FlowControl|Sequence
      (:then_0
        (LocalVariables|SetBeforeRot (Utilities|Array|Get(acopy) _b_hairtailrotations _array_index))
        (Utilities|Array|SetArrayElem _b_hairtailrotations _array_index (.localRotation (Utilities|Struct|BreakSTR_SpringBone _array_element)) true)
        (LocalVariables|SetTemp (.currTipPos (Utilities|Struct|BreakSTR_SpringBone _array_element))))
      (:then_1
        (LocalVariables|SetCurrentTipPos (+ (- (.currTipPos (Utilities|Struct|BreakSTR_SpringBone _array_element)) (.prevTipPos (Utilities|Struct|BreakSTR_SpringBone _array_element))) (.currTipPos (Utilities|Struct|BreakSTR_SpringBone _array_element)) (* (+ (/ (Math|Vector|RotateVector (* (LocalVariables|GetBoneAxis) (.stiffnessForce (Utilities|Struct|BreakSTR_SpringBone _array_element))) (Transformation|GetSocketRotation (Variables|Default|GetSkeletalMesh) (.TargetBone (Utilities|Struct|BreakSTR_SpringBone _array_element)))) _returnvalue_2) (/ (* (- (.prevTipPos (Utilities|Struct|BreakSTR_SpringBone _array_element)) (.currTipPos (Utilities|Struct|BreakSTR_SpringBone _array_element))) (.dragForce (Utilities|Struct|BreakSTR_SpringBone _array_element))) _returnvalue_2) (/ (.springForce (Utilities|Struct|BreakSTR_SpringBone _array_element)) _returnvalue_2)) _returnvalue_2)))
        (LocalVariables|SetCurrentTipPos (+ (* (Math|Vector|Normalize (- (LocalVariables|GetCurrentTipPos) (Transformation|GetSocketLocation (Variables|Default|GetSkeletalMesh) (.TargetBone (Utilities|Struct|BreakSTR_SpringBone _array_element))))) (.SpringLength (Utilities|Struct|BreakSTR_SpringBone _array_element))) (Transformation|GetSocketLocation (Variables|Default|GetSkeletalMesh) (.TargetBone (Utilities|Struct|BreakSTR_SpringBone _array_element))))))
      (:then_2
        (for _array_element_2 (.Colliders (Utilities|Struct|BreakSTR_SpringBone _array_element))
          _)
        (Utilities|Array|SetArrayElem (Variables|/Game/UnityChan/Animations/UnityChanAnimBP.UnityChanAnimBP_C|GetB_HairTailRotations (Variables|Default|GetAnimBP)) _array_index (Math|Rotator|MakeRotator (.Roll (Math|Rotator|BreakRotator (Math|Rotator|Lerp(Rotator) (LocalVariables|GetBeforeRot) (Math|Rotator|CombineRotators (Math|Rotator|FindLookatRotation (Math|Transform|TransformDirection (Transformation|GetSocketTransform _skeletalmesh (.TargetBone (Utilities|Struct|BreakSTR_SpringBone _array_element)) "RTS_World") (LocalVariables|GetBoneAxis)) (- (LocalVariables|GetCurrentTipPos) (Transformation|GetSocketLocation _skeletalmesh (.TargetBone (Utilities|Struct|BreakSTR_SpringBone _array_element))))) (Transformation|GetSocketRotation _skeletalmesh (.TargetBone (Utilities|Struct|BreakSTR_SpringBone _array_element)))) 0.2))) (.Pitch (Math|Rotator|BreakRotator (Math|Rotator|Lerp(Rotator) (LocalVariables|GetBeforeRot) (Math|Rotator|CombineRotators (Math|Rotator|FindLookatRotation (Math|Transform|TransformDirection (Transformation|GetSocketTransform _skeletalmesh (.TargetBone (Utilities|Struct|BreakSTR_SpringBone _array_element)) "RTS_World") (LocalVariables|GetBoneAxis)) (- (LocalVariables|GetCurrentTipPos) (Transformation|GetSocketLocation _skeletalmesh (.TargetBone (Utilities|Struct|BreakSTR_SpringBone _array_element))))) (Transformation|GetSocketRotation _skeletalmesh (.TargetBone (Utilities|Struct|BreakSTR_SpringBone _array_element)))) 0.2))) (.Yaw (Math|Rotator|BreakRotator (.localRotation (Utilities|Struct|BreakSTR_SpringBone _array_element))))) true)
        (Utilities|Array|SetArrayElem (Variables|Default|GetSpringBone_J_B_HairTail) _array_index (Utilities|Struct|MakeSTR_SpringBone (.TargetBone (Utilities|Struct|BreakSTR_SpringBone _array_element)) (LocalVariables|GetCurrentTipPos) (LocalVariables|GetTemp) (.stiffnessForce (Utilities|Struct|BreakSTR_SpringBone _array_element)) (.dragForce (Utilities|Struct|BreakSTR_SpringBone _array_element)) (.springForce (Utilities|Struct|BreakSTR_SpringBone _array_element)) (.SpringLength (Utilities|Struct|BreakSTR_SpringBone _array_element)) (.localRotation (Utilities|Struct|BreakSTR_SpringBone _array_element)) (.Colliders (Utilities|Struct|BreakSTR_SpringBone _array_element))) true)
        (Development|PrintString (Utilities|String|ToString(Rotator) (Math|Rotator|Lerp(Rotator) (LocalVariables|GetBeforeRot) (Math|Rotator|CombineRotators (Math|Rotator|FindLookatRotation (Math|Transform|TransformDirection (Transformation|GetSocketTransform _skeletalmesh (.TargetBone (Utilities|Struct|BreakSTR_SpringBone _array_element)) "RTS_World") (LocalVariables|GetBoneAxis)) (- (LocalVariables|GetCurrentTipPos) (Transformation|GetSocketLocation _skeletalmesh (.TargetBone (Utilities|Struct|BreakSTR_SpringBone _array_element))))) (Transformation|GetSocketRotation _skeletalmesh (.TargetBone (Utilities|Struct|BreakSTR_SpringBone _array_element)))) 0.2)) true true "(R=0.653108,G=1.000000,B=0.760946,A=1.000000)" 0.0)))))