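; BPC_MaterialGear is a component that animates the emissive glow of its owning StaticMeshActor's materials from a curve.
; BeginPlay caches the owner and zeroes the EmissivePower parameter.
; Tick samples TargetCurve at game time plus MusicPlayOffset, scales it by EmissiveLevel and writes it to EmissivePower.
; A pair of gates handles startup: once offset time reaches zero, one opens the glow update and the other shuts off the time check.
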(event EventBeginPlay
  (bind _asstatic_mesh_actor (Utilities|Casting|CastToStaticMeshActor (Components|GetOwner)))
  (Variables|Default|SetStaticMeshActor _asstatic_mesh_actor)
  (Rendering|Material|SetScalarParameterValueonMaterials (Variables|/Script/Engine.StaticMeshActor|GetStaticMeshComponent (Variables|Default|GetStaticMeshActor)) "EmissivePower" 0.0))

(event EventTick
  (params (DeltaSeconds :type Float%20%28single-precision%29))
  (bind _returnvalue (Utilities|Time|GetGameTimeinSeconds))
  (bind _musicplayoffset (Variables|Default|GetMusicPlayOffset))
  (bind _returnvalue_2 (+ _returnvalue _musicplayoffset))
  (Variables|Default|GetStaticMeshActor
    (:then
      (Utilities|FlowControl|Sequence
        (:then_0
          (Utilities|FlowControl|Gate true :!label _label
            (:Exit
              (Rendering|Material|SetScalarParameterValueonMaterials (Variables|/Script/Engine.StaticMeshActor|GetStaticMeshComponent (Variables|Default|GetStaticMeshActor)) "EmissivePower" (* (Math|Curves|GetFloatValue (Variables|Default|GetTargetCurve) _returnvalue_2) (Variables|Default|GetEmissiveLevel))))))
        (:then_1
          (Utilities|FlowControl|Gate false :!label _label_2
            (:Exit
              (if (>= _returnvalue_2 0.0)
                (Utilities|FlowControl|Sequence
                  (:then_0
                    (goto _label Open))
                  (:then_1
                    (goto _label_2 Close)))))))))
    (:else)))