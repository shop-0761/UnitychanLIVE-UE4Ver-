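; Actor component that jitters its owner by adding local location and rotation offsets every tick, scaled per axis and by strength.
; BeginPlay randomises time phases and 2D directions, then opens the Tick gate; frequency-advanced time along each direction feeds Fbm.
; Fbm sums octaves of a Perlin stand-in that is only a clamped linear function, since its random streams always use seed zero.
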(event EventBeginPlay
  (bind _returnvalue (Math|Random|RandomFloat))
  (bind _noisevector (Variables|Default|GetNoiseVector))
  (bind _rotationfractallevel (Variables|Default|GetRotationFractalLevel))
  (bind _noisevector_2 (Variables|Default|GetNoiseVector))
  (bind _locationfractallevel (Variables|Default|GetLocationFractalLevel))
  (bind _returnvalue_2 (Math|Float|MultiplybyPi _returnvalue))
  (bind _returnvalue_3 (* _returnvalue_2 2.0))
  (Variables|Default|SetTimeLocation (* (Math|Random|RandomFloat) 1e+01))
  (Variables|Default|SetTimeRotation (* (Math|Random|RandomFloat) 1e+01))
  (for _index (range 0 6)
    (Utilities|Array|SetArrayElem (Variables|Default|GetNoiseVector) _index (Math|Vector2D|MakeVector2D (Math|Trig|Cos(Radians) _returnvalue_3) (Math|Trig|Sin(Radians) _returnvalue_3)) true))
  (Utilities|FlowControl|Gate true) ; enters at Open
)

(event EventTick
  (params (DeltaSeconds :type Float%20%28single-precision%29))
  (bind _noisevector (Variables|Default|GetNoiseVector))
  (bind _rotationfractallevel (Variables|Default|GetRotationFractalLevel))
  (bind _noisevector_2 (Variables|Default|GetNoiseVector))
  (bind _locationfractallevel (Variables|Default|GetLocationFractalLevel))
  (Utilities|FlowControl|Gate true
    (:Exit
      ;[1 1 1] Location
      (Utilities|FlowControl|Sequence
        (:then_0
          (Variables|Default|SetTimeLocation (+ (Variables|Default|GetTimeLocation) (* DeltaSeconds (Variables|Default|GetLocationFrequency))))
          (if (!= (Variables|Default|GetLocationNoiseStrength) 0.0)
            (Transformation|AddActorLocalOffset (Components|GetOwner) (* (* (* (Variables|Default|GetLocationComponents) (Math|Vector|MakeVector (CallFunction|Fbm (* (Utilities|Array|Get(acopy) _noisevector_2) (Variables|Default|GetTimeLocation)) _locationfractallevel) (CallFunction|Fbm (* (Utilities|Array|Get(acopy) _noisevector_2 1) (Variables|Default|GetTimeLocation)) _locationfractallevel) (CallFunction|Fbm (* (Utilities|Array|Get(acopy) _noisevector_2 2) (Variables|Default|GetTimeLocation)) _locationfractallevel))) (Variables|Default|GetLocationNoiseStrength)) 2.0) false false)))
        (:then_1
          ;[1 1 1] Rotation
          (Variables|Default|SetTimeRotation (+ (Variables|Default|GetTimeRotation) (* DeltaSeconds (Variables|Default|GetRotationFrequency))))
          (if (!= (Variables|Default|GetRotationNoiseStrength) 0.0)
            (Transformation|AddActorLocalRotation (Components|GetOwner) (Math|Rotator|MakeRotator (.X (Math|Vector|BreakVector (* (* (* (Variables|Default|GetRotationComponents) (Math|Vector|MakeVector (CallFunction|Fbm (* (Utilities|Array|Get(acopy) _noisevector 3) (Variables|Default|GetTimeRotation)) _rotationfractallevel) (CallFunction|Fbm (* (Utilities|Array|Get(acopy) _noisevector 4) (Variables|Default|GetTimeRotation)) _rotationfractallevel) (CallFunction|Fbm (* (Utilities|Array|Get(acopy) _noisevector 5) (Variables|Default|GetTimeRotation)) _rotationfractallevel))) (Variables|Default|GetRotationNoiseStrength)) 2.0))) (.Y (Math|Vector|BreakVector (* (* (* (Variables|Default|GetRotationComponents) (Math|Vector|MakeVector (CallFunction|Fbm (* (Utilities|Array|Get(acopy) _noisevector 3) (Variables|Default|GetTimeRotation)) _rotationfractallevel) (CallFunction|Fbm (* (Utilities|Array|Get(acopy) _noisevector 4) (Variables|Default|GetTimeRotation)) _rotationfractallevel) (CallFunction|Fbm (* (Utilities|Array|Get(acopy) _noisevector 5) (Variables|Default|GetTimeRotation)) _rotationfractallevel))) (Variables|Default|GetRotationNoiseStrength)) 2.0))) (.Z (Math|Vector|BreakVector (* (* (* (Variables|Default|GetRotationComponents) (Math|Vector|MakeVector (CallFunction|Fbm (* (Utilities|Array|Get(acopy) _noisevector 3) (Variables|Default|GetTimeRotation)) _rotationfractallevel) (CallFunction|Fbm (* (Utilities|Array|Get(acopy) _noisevector 4) (Variables|Default|GetTimeRotation)) _rotationfractallevel) (CallFunction|Fbm (* (Utilities|Array|Get(acopy) _noisevector 5) (Variables|Default|GetTimeRotation)) _rotationfractallevel))) (Variables|Default|GetRotationNoiseStrength)) 2.0)))) false false)))))))

(fn Fbm
  (params (Coord :type Vector%202D%20Structure) (octave :type Integer))
  (bind _returnvalue (Math|Random|MakeRandomStream 0))
  (bind _returnvalue_2 (Math|Random|RandomFloatfromStream _returnvalue))
  (LocalVariables|SetCoordTemp Coord)
  (LocalVariables|Setf 0.0)
  (LocalVariables|Setw 1.0)
  (for _index (range 0 octave)
    (LocalVariables|Setf (+ (LocalVariables|Getf) (* (LocalVariables|Getw) (- (Math|Float|Clamp(Float) (/ (+ (* (.X (Math|Vector2D|BreakVector2D (LocalVariables|GetCoordTemp))) _returnvalue_2) (* (.Y (Math|Vector2D|BreakVector2D (LocalVariables|GetCoordTemp))) _returnvalue_2)) 2.0)) 0.5))))
    (LocalVariables|SetCoordTemp (* (LocalVariables|GetCoordTemp) 2.0))
    (LocalVariables|Setw (* (LocalVariables|Getw) 0.5)))
  (return (LocalVariables|Getf)))