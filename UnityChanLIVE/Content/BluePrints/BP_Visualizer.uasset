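; BP_Visualizer is a Blueprint that drives a spectrum visualizer material from float curves.
; On BeginPlay it creates a dynamic material instance from the Visualizer component's first material.
; Each Tick it samples the Spectrum1 and Spectrum4 curves at game time and writes them to the red and alpha channels of the Spectra vector parameter.
; A TODO notes intended use of SoundVisualizerPlugin, so no live audio analysis happens here.
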(event EventBeginPlay
  (bind _visualizer (Variables|Default|GetVisualizer))
  (bind _returnvalue (Rendering|Material|CreateDynamicMaterialInstance _visualizer 0 (Rendering|Material|GetMaterial _visualizer 0) "None" :!class /Script/Engine.PrimitiveComponent))
  (Variables|Default|SetDMI_Visualizer _returnvalue))

(event EventTick
  (params (DeltaSeconds :type Float%20%28single-precision%29))
  (bind _returnvalue (Utilities|Time|GetGameTimeinSeconds))
  ;[1 1 1] TODO: Use SoundVisualizerPlugin
  (Rendering|Material|SetVectorParameterValue (Variables|Default|GetDMI_Visualizer) "Spectra" (Math|Color|MakeColor (Math|Curves|GetFloatValue (Variables|Default|GetSpectrum1) _returnvalue) 0.0 0.0 (Math|Curves|GetFloatValue (Variables|Default|GetSpectrum4) _returnvalue)) :!class /Script/Engine.MaterialInstanceDynamic))

(fn ConstructionScript)