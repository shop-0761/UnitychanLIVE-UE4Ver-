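; BP_Spawner is a pooled spawner that repeatedly places and activates actors at target actors while active.
; Init fills the pool with detached child actors, run from the construction script or at BeginPlay if empty.
; Tick accumulates time and triggers spawns at a randomized rate, catching up within one frame.
; Each spawn recycles the next pooled actor round-robin, moves it to a random target, attaches it to any skeletal mesh and sends Activate.
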(event Custom|Init
  (Utilities|Array|Clear (Variables|Default|GetPooledActor))
  (for _index (range 0 (Variables|Default|GetPoolActorNum))
    (bind _returnvalue (AddComponent|AddChildActorComponent false (Math|Transform|MakeTransform "0, 0, 0")))
    (ChildActorComponent|SetChildActorClass _returnvalue (Variables|Default|GetSpawnActor))
    (Transformation|DetachFromActor (Variables|/Script/Engine.ChildActorComponent|GetChildActor _returnvalue) "KeepRelative" "KeepRelative" "KeepRelative")
    (Utilities|Array|Add (Variables|Default|GetPooledActor) (Variables|/Script/Engine.ChildActorComponent|GetChildActor _returnvalue))))

(event EventBeginPlay
  (if (== (Utilities|Array|Length (Variables|Default|GetPooledActor)) 0)
    (CallFunction|Init)))

(event EventTick
  (params (DeltaSeconds :type Float%20%28single-precision%29))
  ;[1 1 1] Tick
  (if (Variables|Default|GetIsActive)
    (Variables|Default|SetTimer (+ DeltaSeconds (Variables|Default|GetTimer)))
    (while (> (Variables|Default|GetTimer) (/ (- 1.0 (Variables|Default|GetRandomValue)) (Variables|Default|GetSpawnRate)))
      (CallFunction|SpawnPooledActor)
      (Variables|Default|SetTimer (- (Variables|Default|GetTimer) (/ (- 1.0 (Variables|Default|GetRandomValue)) (Variables|Default|GetSpawnRate))))
      (Variables|Default|SetRandomValue (* (Math|Random|RandomFloat) (Variables|Default|GetSpawnRateRondomness))))))

(fn ConstructionScript
  (CallFunction|Init))

(fn SpawnPooledActor
  (bind _targetactors (Variables|Default|GetTargetActors))
  (bind _returnvalue (Utilities|Array|Length _targetactors))
  (LocalVariables|SetSpawnPointIndex (Math|Integer|%(Integer) (+ (LocalVariables|GetSpawnPointIndex) (Math|Random|RandomIntegerinRange 1 _returnvalue)) _returnvalue))
  (Transformation|SetActorTransform (Utilities|Array|Get(acopy) (Variables|Default|GetPooledActor) (Variables|Default|GetPooledIndex)) (Transformation|GetActorTransform (Utilities|Array|Get(acopy) (Variables|Default|GetTargetActors) (LocalVariables|GetSpawnPointIndex))))
  (Utilities|IsValid (Actor|GetComponentbyClass (Utilities|Array|Get(acopy) (Variables|Default|GetTargetActors) (LocalVariables|GetSpawnPointIndex)) "/Script/Engine.SkeletalMeshComponent")
    (:Is%20Valid
      (Transformation|AttachComponentToComponent (Utilities|Array|Get(acopy) (Variables|Default|GetPooledActor) (Variables|Default|GetPooledIndex)) (Actor|GetComponentbyClass (Utilities|Array|Get(acopy) (Variables|Default|GetTargetActors) (LocalVariables|GetSpawnPointIndex)) "/Script/Engine.SkeletalMeshComponent") "None" "SnapToTarget" "SnapToTarget" "KeepWorld" true))
    (:Is%20Not%20Valid
      _))
  (Class|BPISpawnableActor|Activate(Message) (Utilities|Array|Get(acopy) (Variables|Default|GetPooledActor) (Variables|Default|GetPooledIndex)))
  (Variables|Default|SetPooledIndex (Math|Integer|%(Integer) (+ (Variables|Default|GetPooledIndex) 1) (Utilities|Array|Length (Variables|Default|GetPooledActor)))))