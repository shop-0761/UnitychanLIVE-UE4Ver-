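; Camera switcher that cuts MainCamera between target points, automatically on an interval when enabled, while keeping it aimed at a target actor's CameraTarget socket.
; Default mode starts at the first point then picks randomly, sometimes offsetting aim by Stability; GameInstance's demo flag selects predefined point sequences and, for cine cameras, aim offsets.
; Tick exponentially eases aim back onto the socket.
; Each cut sets cine focal length from a distance-based FOV curve.
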(event Custom|StopAutoChange
  ;[1 1 1] Auto Change
  (Variables|Default|SetIsAutoChange false)
  (Variables|Default|SetInterval 0.0)
  (Utilities|FlowControl|RetriggerableDelay (Variables|Default|GetInterval) :!label _label)
  (if (Variables|Default|GetIsAutoChange)
    (bind _return (Utilities|ChooseAnotherPoint (Variables|Default|GetTargetPoints) (Variables|Default|GetIsDemo)))
    (CallFunction|ChangeLocation _return)
    (goto _label)))

(event Custom|ChangeLocation
  (params (Destination :type Vector))
  (bind _cinecameraactor (Variables|Default|GetCineCameraActor))
  (bind _returnvalue (Class|CineCameraActor|GetCineCameraComponent _cinecameraactor))
  ;[1 1 1] ChangeLocation
  (Transformation|SetActorLocation (Variables|Default|GetMainCamera) Destination false false)
  (Utilities|FlowControl|Sequence
    (:then_0
      (bind _skeletalmeshcomponent (Variables|Default|GetSkeletalMeshComponent)
        (:then
          (if (and (Variables|Default|GetIsDemo) (Variables|Default|GetIsCineCameraActor))
            ;;[1 1 1] Demo
            (bind _item (Utilities|GetNextItem (Variables|Demo|GetDemoCameraLocRandomIndex)))
            (Variables|Default|SetFollowPoint (+ _item (Transformation|GetSocketLocation _skeletalmeshcomponent "CameraTarget")))
            (else
              ;;[1 1 1] Default
              (if (> (Variables|Default|Getstability) (Math|Random|RandomFloat))
                (Variables|Default|SetFollowPoint (Transformation|GetSocketLocation _skeletalmeshcomponent "CameraTarget"))
                (else
                  (Variables|Default|SetFollowPoint (+ (Transformation|GetSocketLocation _skeletalmeshcomponent "CameraTarget") (* (Math|Random|RandomUnitVector) (Math|Random|RandomFloatinRange 0.0 5e+02)))))))))
        (:else)))
    (:then_1
      (if (Variables|Default|GetIsCineCameraActor)
        (Variables|/Script/CinematicCamera.CineCameraComponent|SetCurrentFocalLength _returnvalue (/ (/ (.sensorwidth (Variables|/Script/CinematicCamera.CineCameraComponent|GetFilmbackSettings _returnvalue)) 2.0) (Math|Trig|Tan(Radians) (/ (Math|Trig|DegreesToRadians (* (Math|Curves|GetFloatValue (Variables|Default|GetFOVCurve) (/ (Math|Vector|VectorLength (- (Transformation|GetActorLocation (Variables|Default|GetMainCamera)) (Transformation|GetActorLocation (Variables|Default|GetTargetActor)))) 1e+02)) (Variables|Default|GetFOVPower))) 2.0))))))))

(event Custom|AutoChange
  ;[1 1 1] Auto Change
  (Variables|Default|SetIsAutoChange true)
  (Variables|Default|SetInterval (Variables|Default|GetDefaultInterval))
  (if (Variables|Default|GetIsAutoChange) :!label _label
    (bind _return (Utilities|ChooseAnotherPoint (Variables|Default|GetTargetPoints) (Variables|Default|GetIsDemo)))
    (CallFunction|ChangeLocation _return)
    (Utilities|FlowControl|RetriggerableDelay (Variables|Default|GetInterval))
    (goto _label)))

(event EventTick
  (params (DeltaSeconds :type Float%20%28single-precision%29))
  (bind _maincamera (Variables|Default|GetMainCamera))
  ;[1 1 1] Tick
  (bind _skeletalmeshcomponent (Variables|Default|GetSkeletalMeshComponent)
    (:then
      (Variables|Default|SetFollowPoint (Math|Vector|Lerp(Vector) (Transformation|GetSocketLocation _skeletalmeshcomponent "CameraTarget") (Variables|Default|GetFollowPoint) (Class|KismetMathLibrary|Exp (* DeltaSeconds (* (Variables|Default|GetrotationSpeed) -1.0)))))
      (Transformation|SetActorRotation _maincamera (Math|Rotator|FindLookatRotation (Transformation|GetActorLocation _maincamera) (Variables|Default|GetFollowPoint)) true))
    (:else)))

(event EventBeginPlay
  (bind _maincamera (Variables|Default|GetMainCamera))
  (bind (_ascine_camera_actor _bsuccess) (Utilities|Casting|CastToCineCameraActor _maincamera))
  ;[1 1 1] BeginPlay
  (bind _targetactor (Variables|Default|GetTargetActor)
    (:then
      (Utilities|IsValid (Actor|GetComponentbyClass _targetactor "/Script/Engine.SkeletalMeshComponent")
        (:Is%20Valid
          (bind _output_get (Variables|Default|SetSkeletalMeshComponent (Actor|GetComponentbyClass _targetactor "/Script/Engine.SkeletalMeshComponent")))
          (Variables|Default|SetFollowPoint (Transformation|GetSocketLocation _output_get "CameraTarget"))
          (Variables|Default|SetDefaultInterval (Variables|Default|GetInterval))
          (Utilities|FlowControl|Sequence
            (:then_0
              (if (Variables|Default|GetIsAutoChange)
                (CallFunction|AutoChange)))
            (:then_1
              (bind _asbp_game_instance (Utilities|Casting|CastToBP_GameInstance (Game|GetGameInstance)))
              (Variables|Default|SetIsDemo (Variables|/Game/BluePrints/BP_GameInstance.BP_GameInstance_C|GetIsDemo _asbp_game_instance)))
            (:then_2
              (Variables|Default|SetCineCameraActor _ascine_camera_actor)
              (Variables|Default|SetIsCineCameraActor _bsuccess))))))
    (:else)))

(fn ConstructionScript)