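; Actor component that cuts its owning camera between target points while keeping it aimed at the target actor's CameraTarget socket.
; Tick turns the camera toward a follow point eased by framerate-independent exponential smoothing, which each cut resets, with random offset depending on Stability.
; An auto-change loop moves it every Interval seconds through a scripted demo index order; ChooseAnotherPoint's unused non-demo branch picks randomly after the first point.
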(event Custom|StopAutoChange
  (Variables|Default|SetIsAutoChange false)
  (Variables|Default|SetInterval 0.0)
  (Utilities|FlowControl|RetriggerableDelay (Variables|Default|GetInterval) :!label _label)
  (if (Variables|Default|GetIsAutoChange)
    (bind _return (Utilities|ChooseAnotherPoint (Variables|Default|GetTargetPoints) true))
    (CallFunction|ChangeLocation _return)
    (goto _label)))

(event Custom|ChangeLocation
  (params (Destination :type Vector))
  (Transformation|SetActorLocation (Variables|Default|GetCamera) Destination false false)
  (bind _skeletalmeshcomponent (Variables|Default|GetSkeletalMeshComponent)
    (:then
      (if (> (Variables|Default|Getstability) (Math|Random|RandomFloat))
        (Variables|Default|SetFollowPoint (Transformation|GetSocketLocation _skeletalmeshcomponent "CameraTarget"))
        (else
          (Variables|Default|SetFollowPoint (+ (Transformation|GetSocketLocation _skeletalmeshcomponent "CameraTarget") (* (Math|Random|RandomUnitVector) (Math|Random|RandomFloatinRange 0.0 5.0)))))))
    (:else)))

(event Custom|AutoChange_Main
  (Variables|Default|SetIsAutoChange true)
  (Variables|Default|SetInterval (Variables|Default|GetDefaultInterval))
  (if (Variables|Default|GetIsAutoChange) :!label _label
    (bind _return (Utilities|ChooseAnotherPoint (Variables|Default|GetTargetPoints) true))
    (CallFunction|ChangeLocation _return)
    (Utilities|FlowControl|RetriggerableDelay (Variables|Default|GetInterval))
    (goto _label)))

(event EventBeginPlay
  ;[1 1 1] BeginPlay
  (Variables|Default|SetCamera (Components|GetOwner))
  (bind _targetactor (Variables|Default|GetTargetActor)
    (:then
      (Utilities|IsValid (Actor|GetComponentbyClass _targetactor "/Script/Engine.SkeletalMeshComponent")
        (:Is%20Valid
          (bind _output_get (Variables|Default|SetSkeletalMeshComponent (Actor|GetComponentbyClass _targetactor "/Script/Engine.SkeletalMeshComponent")))
          (Variables|Default|SetFollowPoint (Transformation|GetSocketLocation _output_get "CameraTarget"))
          (Variables|Default|SetDefaultInterval (Variables|Default|GetInterval)))))
    (:else)))

(event EventTick
  (params (DeltaSeconds :type Float%20%28single-precision%29))
  (bind _camera (Variables|Default|GetCamera))
  ;[1 1 1] UpdateCameraRot
  (bind _skeletalmeshcomponent (Variables|Default|GetSkeletalMeshComponent)
    (:then
      (Variables|Default|SetFollowPoint (Math|Vector|Lerp(Vector) (Transformation|GetSocketLocation _skeletalmeshcomponent "CameraTarget") (Variables|Default|GetFollowPoint) (Class|KismetMathLibrary|Exp (* DeltaSeconds (* (Variables|Default|GetrotationSpeed) -1.0)))))
      (Transformation|SetActorRotation _camera (Math|Rotator|FindLookatRotation (Transformation|GetActorLocation _camera) (Variables|Default|GetFollowPoint)) true))
    (:else)))